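; Player controller for LeaveMeAlone that opens the pause menu when the Pause input is pressed.
; An OnPause flag blocks repeat presses and is not cleared in this graph.
; If the player character has an LMAWeaponComponent, it stops firing before the game pauses.
; It then creates and displays WBP_Pause, switches input to UI-only focused on that widget and shows the mouse cursor.
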(event EventBeginPlay)

(event EventTick
  (params (DeltaSeconds :type Float%20%28single-precision%29)))

(event Input|ActionEvents|InputActionPause
  (params (Key :type Key%20Structure :default "None"))
  (bind _returnvalue (Game|GetPlayerCharacter 0))
  (bind _returnvalue_2 (Actor|GetComponentbyClass _returnvalue "/Script/LeaveMeAlone.LMAWeaponComponent"))
  (:Pressed
    (if (not (Variables|Default|GetOnPause))
      (Variables|Default|SetOnPause true)
      (Utilities|IsValid _returnvalue
        (:Is%20Valid
          (Utilities|IsValid _returnvalue_2
            (:Is%20Valid
              (Class|LMAWeaponComponent|StopFire _returnvalue_2)
              (Game|SetGamePaused true)
              (bind _returnvalue_3 (UserInterface|CreateWidget "/Game/LeaveMeAlone/Widgets/UI/WBP_Pause.WBP_Pause_C"))
              (bind _output_get (Variables|Default|SetPauseWidget _returnvalue_3))
              (UserInterface|Viewport|AddtoViewport _output_get 0)
              (Input|SetInputModeUIOnly self _output_get "DoNotLock" false)
              (Variables|Default|SetbShowMouseCursor true))))))))

(fn ConstructionScript)