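; Game mode for LeaveMeAlone that runs a survival countdown and decides win or loss.
; On BeginPlay a looping one-second timer decrements GameTime, and the player character's health component death event is bound to the loss flow.
; Time reaching zero shows the win widget, while death shows the loss widget after a short delay.
; Both outcomes call StopControl, which clears the timer, pauses the game and switches to UI-only input with a visible cursor.
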(event Custom|TimeEvent
  (bind _output_get (Variables|Default|SetGameTime (- (Variables|Default|GetGameTime) 1)))
  (if (== _output_get 0)
    (CallFunction|StopControl)
    (bind _returnvalue (UserInterface|CreateWidget "/Game/LeaveMeAlone/Widgets/UI/WBP_GameWin.WBP_GameWin_C"))
    (UserInterface|Viewport|AddtoViewport _returnvalue 0)))

(event Custom|ViewLossWidget
  (Utilities|FlowControl|Delay 1.5)
  (CallFunction|StopControl)
  (bind _returnvalue (UserInterface|CreateWidget "/Game/LeaveMeAlone/Widgets/UI/WBP_GameLoss.WBP_GameLoss_C"))
  (UserInterface|Viewport|AddtoViewport _returnvalue 0))

(event EventBeginPlay
  (bind _returnvalue (Utilities|Time|SetTimerbyEvent (delegate Custom|TimeEvent) 1.0 true))
  (Variables|Default|SetGameTimerHandle _returnvalue)
  (EventDispatchers|BindEventtoOnDeath (Actor|GetComponentbyClass (Game|GetPlayerCharacter 0) "/Script/LeaveMeAlone.LMAHealthComponent") (delegate Custom|ViewLossWidget)))

(event EventTick
  (params (DeltaSeconds :type Float%20%28single-precision%29)))

(fn ConstructionScript)

(fn StopControl
  (bind _returnvalue (Game|GetPlayerController 0))
  (Utilities|Time|ClearandInvalidateTimerbyHandle (Variables|Default|GetGameTimerHandle))
  (Game|SetGamePaused true)
  (Input|SetInputModeUIOnly _returnvalue 0 "DoNotLock" false)
  (Variables|/Script/Engine.PlayerController|SetbShowMouseCursor _returnvalue true))